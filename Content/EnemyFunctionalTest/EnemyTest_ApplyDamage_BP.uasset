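; Functional test that checks an enemy's claw swing actually deals damage to the character.
; It records the character's starting Health, then has player controller 0 possess the character when the test starts.
; Each tick, once the Enemy's CombatCollision overlaps the character, it passes if Health has dropped below the start value and fails otherwise.
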(event `self.ReceivePrepareTest`
  ;[1 1 1] Get Character's start health
  (bind _character (`self.Character`)
    (:`then`
      (set `self.CharacterStartHealth` (`MainCharacter.Health` _character)))
    (:`else`)))

(event `self.ReceiveStartTest`
  (`Controller.Possess` (`GameplayStatics.GetPlayerController` 0) (`self.Character`)))

(event `self.ReceiveTick`
  (params (DeltaSeconds :type "Float (single-precision)"))
  ;[1 1 1] Check if Enemy apply damagae to Character when Enemy's swinging its claw and overlapping the character (the claw has CombatCollision attached).
  (if (`PrimitiveComponent.IsOverlappingActor` (`Enemy.CombatCollision` (`self.Enemy`)) (`self.Character`))
    (if (< (`MainCharacter.Health` (`self.Character`)) (`self.CharacterStartHealth`))
      (`self.FinishTest` "Succeeded" "Enemy's claw actually apply damage to the Character")
      (else
        (`self.FinishTest` "Failed" "Enemy's claw Does Not apply damage to the Character")))))

(fn `UserConstructionScript`)