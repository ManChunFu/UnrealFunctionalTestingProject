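; Functional test that verifies an enemy plays its death animation when its health runs out.
; On start it possesses the test character, gives the weapon lethal damage, equips it, attacks, and records the enemy's current montage section.
; On tick, once enemy health reaches zero or below, it passes only if the montage section has changed to "Death", otherwise it fails.
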(event `self.ReceiveStartTest`
  (bind _character (`self.Character`)
    (:`then`
      (`Controller.Possess` (`GameplayStatics.GetPlayerController` 0) _character)
      ;[1 1 1] Setup Weapon's damage to 100 and let Character to euip and swing the blade. Then get Enemy's start animtion montage section.
      (bind _weapon (`self.Weapon`)
        (:`then`
          (set `Weapon.Damage` 100.0 _weapon)
          (`Weapon.Equip` _weapon (`self.Character`))
          (`MainCharacter.Attack` (`self.Character`))
          (bind _enemy (`self.Enemy`)
            (:`then`
              (bind _returnvalue (`SkeletalMeshComponent.GetAnimInstance` (`Character.Mesh` _enemy)))
              (set `self.EnemyStartMontageSection` (`AnimInstance.Montage_GetCurrentSection` _returnvalue (`AnimInstance.GetCurrentActiveMontage` _returnvalue))))
            (:`else`)))
        (:`else`)))
    (:`else`)))

(event `self.ReceiveTick`
  (params (DeltaSeconds :type "Float (single-precision)"))
  (bind _returnvalue (`SkeletalMeshComponent.GetAnimInstance` (`Character.Mesh` (`self.Enemy`))))
  (bind _returnvalue_2 (`AnimInstance.Montage_GetCurrentSection` _returnvalue (`AnimInstance.GetCurrentActiveMontage` _returnvalue)))
  ;[1 1 1] Check if Enemy's anim instance does jump montage to "Death" section when its health is less or equal 0.
  (if (<= (`Enemy.Health` (`self.Enemy`)) 0.0)
    (if (and (!= (`self.EnemyStartMontageSection`) _returnvalue_2) (== _returnvalue_2 "Death"))
      (`self.FinishTest` "Succeeded" "Enemy does play Death animation when the health is 0")
      (else
        (`self.FinishTest` "Failed" "Enemy does NOT play Death animation when the health is 0")))))

(fn `UserConstructionScript`)