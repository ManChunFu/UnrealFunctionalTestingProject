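; Functional test Blueprint that checks an enemy moves toward the player character when that character overlaps its AgroSphere.
; On start it possesses the character, then passes the first overlapping actor, cast to MainCharacter_BP, to the enemy's MoveToTarget, or fails if the character is not overlapping.
; Tick passes the test once the enemy is within a fixed distance of the character.
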(event `self.ReceivePrepareTest`)

(event `self.ReceiveStartTest`
  (bind _agrosphere (`Enemy.AgroSphere` (`self.Enemy`)))
  ;[1 1 1] Check if Enemy's"MoveToTarget" function get triggerred when character(target) is overlapping Enemy's AgroSphereComponent
  (`Controller.Possess` (`GameplayStatics.GetPlayerController` 0) (`self.Character`))
  (if (`PrimitiveComponent.IsOverlappingActor` _agrosphere (`self.Character`))
    (bind _asmain_character_bp (cast `/Game/Character/MainCharacter_BP` (`|GetArrayItem` (`PrimitiveComponent.GetOverlappingActors` _agrosphere null))))
    (`Enemy.MoveToTarget` (`self.Enemy`) _asmain_character_bp)
    (else
      (`self.FinishTest` "Failed" "Need an Actor/Character to trigger move to target function"))))

(event `self.ReceiveTick`
  (params (DeltaSeconds :type "Float (single-precision)"))
  ;[1 1 1] Check if Enemy really moves to the target (current location) that was fed from overlapping to "MoveToTarget" function.
  (bind _enemy (`self.Enemy`)
    (:`then`
      (if (< (`KismetMathLibrary.VSize` (- (`self.K2_GetActorLocation` _enemy) (`self.K2_GetActorLocation` (`self.Character`)))) 200.0)
        (`self.FinishTest` "Succeeded" "Enemy does move toward to the character")))
    (:`else`)))

(fn `UserConstructionScript`)