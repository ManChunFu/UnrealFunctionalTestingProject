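; Functional test that checks whether an Enemy switches to its combat montage when the test Character enters its CombatSphere.
; On start it possesses the Character with player controller 0 and records the Enemy's current montage as a baseline.
; Tick waits for the sphere overlap, then immediately passes only if the montage differs from the baseline and equals SpiderCombatMontage, otherwise it fails.
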(event `self.ReceivePrepareTest`)

(event `self.ReceiveStartTest`
  (bind _character (`self.Character`)
    (:`then`
      (`Controller.Possess` (`GameplayStatics.GetPlayerController` 0) _character)
      ;[1 1 1] Get the Enemy's current montage when no actor/character is overlapping CombatSphereComponent.
      (bind _returnvalue (`Character.GetCurrentMontage` (`self.Enemy`)))
      (set `self.EnemyStartMontage` _returnvalue))
    (:`else`)))

(event `self.ReceiveTick`
  (params (DeltaSeconds :type "Float (single-precision)"))
  ;[1 1 1] Check if Enemy switch to combat mode when its CombatSphereComponent is overlapping an actor/Character.
  (if (`PrimitiveComponent.IsOverlappingActor` (`Enemy.CombatSphere` (`self.Enemy`)) (`self.Character`))
    (bind _returnvalue (`Character.GetCurrentMontage` (`self.Enemy`)))
    (if (and (!= _returnvalue (`self.EnemyStartMontage`)) (== _returnvalue "/Game/Enemies/Spider/SpiderCombatMontage.SpiderCombatMontage"))
      (`self.FinishTest` "Succeeded" "Enemy does change to Combat Montage animation")
      (else
        (`self.FinishTest` "Failed" "Enemy doesn't change to Combat Montage animation")))))

(fn `UserConstructionScript`)