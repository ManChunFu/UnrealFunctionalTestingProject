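; FloorSwitch_BP is a floor switch Blueprint that animates a pressure switch and the door paired with it.
; Lower and raise events play or reverse separate switch and door timelines.
; Each timeline feeds its elevation curve to an update-location function defined outside this graph.
; When the door timeline finishes while IsOpening is true, IsDoorFullyOpened is set.
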(event `self.LowerFloorSwitch`
  (bind (_direction _floorswitchelevation) (`Timeline|FloorSwitchTimeline` :`NewTime` (`GameplayStatics.GetWorldDeltaSeconds`) :!label _label)
    (:`Update`
      (`self.UpdateFloorSwitchLocation` _floorswitchelevation))))

(event `self.RaiseFloorSwitch`
  (goto _label :!via `Reverse`))

(event `self.RaiseDoor`
  (bind (_direction _doorelevation) (`Timeline|DoorTimeline` :`NewTime` (`GameplayStatics.GetWorldDeltaSeconds`) :!label _label_2)
    (:`Update`
      (`self.UpdateDoorLocation` _doorelevation))
    (:`Finished`
      (if (`self.IsOpening`)
        (set `self.bIsDoorFullyOpened` true)))))

(event `self.LowerDoor`
  (goto _label_2 :!via `Reverse`))

(fn `UserConstructionScript`)